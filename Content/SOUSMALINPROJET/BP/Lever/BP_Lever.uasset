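; VR grabbable lever that switches the drill activity on and off through BGI_Game, with a looping or one-off sound.
; While grabbed, a timer rolls the pivot toward the motion controller, and on release the pivot snaps to its min or max angle.
; Tick derives the active state from a box overlapping the trigger.
; An electricity shutdown forces it off with a timeline animation; the roll clamp is never executed.
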(event `self.ReceiveBeginPlay`
  (bind _pivot (`self.Pivot`))
  (bind (_relativerotation_roll _relativerotation_pitch _relativerotation_yaw) (`KismetMathLibrary.BreakRotator` (`SceneComponent.RelativeRotation` _pivot)))
  ;[1 1 1] Initializing
  (`SceneComponent.K2_SetRelativeRotation` _pivot (`KismetMathLibrary.MakeRotator` (`self.MinAmplitude`) _relativerotation_pitch _relativerotation_yaw) false false)
  (set `self.IsLeverActive` false)
  (`SceneComponent.K2_SetWorldLocation` (`self.Audio`) (`self.SoundLocation`) false true)
  (add `ElectricitySubsystem.OnShutDown` (subsystem `ElectricitySubsystem`) (delegate `EC_TurnOff`))
  (bind _asbgi_game (cast `/Game/SOUSMALINPROJET/BP/Game/BGI_Game` (`GameplayStatics.GetGameInstance`)))
  (set `self.GameInstance` _asbgi_game)
  (add `/Game/VRTemplate/Blueprints/GrabComponent.OnDropped` (`self.GrabComponent`) (delegate `EC_Drop`)))

(event `self.GrabComponent.OnGrabbed`
  (params (`Motion controller` :type "MotionControllerComponent Object Reference"))
  (set `self.Motion Controller` `Motion controller`)
  (bind _returnvalue (`KismetSystemLibrary.K2_SetTimerDelegate` (delegate `UpdateRotation`) 0.02 true)))

(event `EC_Drop`
  (`self.Dropped`))

(event `EC_TurnOff`
  ;[1 1 1] Initializing
  (`self.TurnOff`))

(event `self.ReceiveTick`
  (params (DeltaSeconds :type "Float (single-precision)"))
  (bind _isleveractive (`self.IsLeverActive`))
  (bind _isleveractive_2 (`self.IsLeverActive`))
  (bind _audio (`self.Audio`))
  (`|ExecutionSequence`
    (:`then_1`
      ;[1 1 1] Update State
      (if (`PrimitiveComponent.IsOverlappingComponent` (`self.BoxTrigger`) (`self.Box`))
        (if (not _isleveractive)
          (set `self.IsLeverActive` true)
          (`/Game/SOUSMALINPROJET/BP/Game/BGI_Game.DrillActivity` (`self.GameInstance`) _isleveractive_2 :!label _label)
          ;[1 1 1] Sound Trigger
          (if _isleveractive_2
            (`AudioComponent.Play` _audio 0.0)
            (else
              (`AudioComponent.Stop` _audio))))
        (elif _isleveractive
          (set `self.IsLeverActive` false)
          (goto _label))))))

(event `UpdateRotation`
  (bind _output_get (set `self.CurrentValue` (`KismetMathLibrary.FInterpTo` (`self.CurrentValue`) (* (`KismetMathLibrary.NormalizeAxis` (`KismetMathLibrary.Dot_VectorVector` (`KismetMathLibrary.Conv_RotatorToVector` (`KismetMathLibrary.FindLookAtRotation` (`SceneComponent.K2_GetComponentLocation` (`self.Pivot`)) (`SceneComponent.K2_GetComponentLocation` (`self.Motion Controller`)))) (`KismetMathLibrary.GetRightVector` (`SceneComponent.K2_GetComponentRotation` (`self.Pivot`))))) 100.0) (`KismetSystemLibrary.K2_GetTimerElapsedTimeHandle` (stale `self.GrabComponent.OnGrabbed` _returnvalue)))))
  (`SceneComponent.K2_AddLocalRotation` (`self.Pivot`) (`KismetMathLibrary.MakeRotator` _output_get) false false))

(event `Dropped`
  (bind _pivot (`self.Pivot`))
  (bind (_relativerotation_roll _relativerotation_pitch _relativerotation_yaw) (`KismetMathLibrary.BreakRotator` (`SceneComponent.RelativeRotation` _pivot)))
  (if (`self.IsLeverActive`)
    (`SceneComponent.K2_SetRelativeRotation` _pivot (`KismetMathLibrary.MakeRotator` (`self.MaxAmplitude`) _relativerotation_pitch _relativerotation_yaw) false false)
    (else
      (`SceneComponent.K2_SetRelativeRotation` _pivot (`KismetMathLibrary.MakeRotator` (`self.MinAmplitude`) _relativerotation_pitch _relativerotation_yaw) false false))))

(event `self.GrabComponent.OnDropped`
  (set `self.Motion Controller` null)
  (`KismetSystemLibrary.K2_PauseTimer` null "UpdateRotation"))

(event `TurnOff`
  (bind _pivot (`self.Pivot`))
  (bind (_relativerotation_roll _relativerotation_pitch _relativerotation_yaw) (`KismetMathLibrary.BreakRotator` (`SceneComponent.RelativeRotation` _pivot)))
  (bind _output_get (set `self.IsLeverActive` false))
  (`/Game/SOUSMALINPROJET/BP/Game/BGI_Game.DrillActivity` (`self.GameInstance`) _output_get)
  (bind (_direction _newtrack_0) (`Timeline|TurnOffAnim`)
    (:`Update`
      (`SceneComponent.K2_SetRelativeRotation` _pivot (`KismetMathLibrary.MakeRotator` (`KismetMathLibrary.Lerp` _relativerotation_roll (`self.MinAmplitude`) _newtrack_0) _relativerotation_pitch _relativerotation_yaw) false false))))

(fn `UserConstructionScript`)