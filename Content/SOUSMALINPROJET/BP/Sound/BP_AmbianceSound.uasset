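; BP_AmbianceSound plays a recurring ambient sound at random positions around the player pawn.
; PlaySound stores the ambiance data and starts a timer with a random delay between that data's min and max play times.
; Each time the timer fires, it plays the sound with its volume and ambiance attenuation at a random direction and set radius from the pawn, then re-arms the timer with a new delay.
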(event `self.ReceiveBeginPlay`
  ;[1 1 1] Main Pawn
  (set `self.MainPawn` (`GameplayStatics.GetPlayerPawn` 0)))

(event `PlaySound`
  (params (AmbianceData :type "/Game/SOUSMALINPROJET/BP/Sound/S_AmbianceMusic Structure"))
  (bind _output_get (set `self.Ambiance Data` AmbianceData))
  (bind _randomduration (`self.GetSoundDuration` _output_get :!label _label))
  (`KismetSystemLibrary.K2_SetTimerDelegate` (delegate `SoundPlay`) _randomduration))

(event `SoundPlay`
  (`self.PlayAmbianceSound` (`self.Ambiance Data`))
  (goto _label))

(fn `GetSoundDuration`
  (params (AmbianceData :type "/Game/SOUSMALINPROJET/BP/Sound/S_AmbianceMusic Structure"))
  (returns (RandomDuration :type "Float (double-precision)"))
  (locals (Random :type "Float (double-precision)"))
  (bind (_sound _minplaytime _maxplaytime) (break `/Game/SOUSMALINPROJET/BP/Sound/S_AmbianceMusic` AmbianceData))
  (bind _output_get (set `local.Random` (`KismetMathLibrary.RandomFloatInRange` _minplaytime _maxplaytime)))
  (return _output_get))

(fn `PlayAmbianceSound`
  (params (AmbianceData :type "/Game/SOUSMALINPROJET/BP/Sound/S_AmbianceMusic Structure"))
  (bind (_sound _minplaytime _maxplaytime _volume) (break `/Game/SOUSMALINPROJET/BP/Sound/S_AmbianceMusic` AmbianceData))
  (`GameplayStatics.PlaySoundAtLocation` _sound (+ (`self.K2_GetActorLocation` (`self.MainPawn`)) (* (`KismetMathLibrary.RandomUnitVector`) (`self.Radius`))) (struct) _volume 1.0 0.0 "/Game/SOUSMALINPROJET/BP/Sound/ATT_Ambiance.ATT_Ambiance" null null null))

(fn `UserConstructionScript`)