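; BP_MonsterManager controls when the big monster spawns, attacks and retreats in response to light switching.
; On BeginPlay it sets the ElectricitySubsystem's power and binds to its light-switch delegate.
; A true callback makes the existing monster attack, or starts a cooldown timer that spawns one on a circle around world origin, passes MonsterData and attacks.
; A false callback cancels that timer and calls EscapeAndWait on the monster.
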(event `self.ReceiveBeginPlay`
  (set `ElectricitySubsystem.CurrentPower` 1000.0 (subsystem `ElectricitySubsystem`))
  (add `ElectricitySubsystem.OnLightSwitched` (subsystem `ElectricitySubsystem`) (delegate `ActivityTrigger`)))

(event `ECSpawnBigMonster`
  (`self.SpawnBigMonster`))

(event `ActivityTrigger`
  (params (Callback :type Boolean))
  (if Callback
    (`self.BigMonsterRef`
      (:`then`
        (`/Game/SOUSMALINPROJET/BP/BP_Monster/BP_BigMonster.Attack` (`self.BigMonsterRef`)))
      (:`else`
        (bind _returnvalue (`KismetSystemLibrary.K2_SetTimerDelegate` (delegate `ECSpawnBigMonster`) (`self.SpawnCooldown`)))
        (set `self.SpawnTimerHandle` _returnvalue)))
    (else
      (if (`KismetSystemLibrary.K2_IsValidTimerHandle` (`self.SpawnTimerHandle`))
        (`KismetSystemLibrary.K2_ClearAndInvalidateTimerHandle` (`self.SpawnTimerHandle`)))
      (`/Game/SOUSMALINPROJET/BP/BP_Monster/BP_BigMonster.EscapeAndWait` (`self.BigMonsterRef`)))))

(event `SpawnBigMonster`
  (bind _randompositioninradius (`self.GetRandomPointInRadius`))
  (bind _returnvalue (`|SpawnActorFromClass` "/Game/SOUSMALINPROJET/BP/BP_Monster/BP_BigMonster.BP_BigMonster_C" (`KismetMathLibrary.MakeTransform` _randompositioninradius) "Undefined" "MultiplyWithRoot" null null))
  (bind _output_get (set `self.BigMonsterRef` _returnvalue))
  (set `/Game/SOUSMALINPROJET/BP/BP_Monster/BP_BigMonster.MonsterData` (`self.MonsterData`) _output_get)
  (`/Game/SOUSMALINPROJET/BP/BP_Monster/BP_BigMonster.Attack` (`self.BigMonsterRef`)))

(fn `GetRandomPointInRadius`
  (returns (RandomPositionInRadius :type "Vector Structure"))
  (locals (RandomAngle :type "Float (double-precision)"))
  (bind _output_get (set `local.RandomAngle` (* (`KismetMathLibrary.MultiplyByPi` (`KismetMathLibrary.RandomFloat`)) 2.0)))
  (return (`KismetMathLibrary.MakeVector` (* (`KismetMathLibrary.Cos` _output_get) (`self.RadiusSpawn`)) (* (`KismetMathLibrary.Sin` _output_get) (`self.RadiusSpawn`)))))

(fn `UserConstructionScript`)