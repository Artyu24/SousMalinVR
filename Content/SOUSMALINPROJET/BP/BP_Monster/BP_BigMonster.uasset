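; BP_BigMonster is a monster that advances on a destination, repeatedly attacks there, and later escapes.
; Attack loads MonsterData and plays a speed-scaled timeline, lerping from the current location toward the destination each update.
; Within proximity radius, it stops and starts a looping timer calling OnHit on BGI_Game.
; EscapeAndWait cancels that timer, then after a delay reverses the timeline and destroys the actor on finish, unless Attack interrupts.
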(event `Attack`
  (bind (_monsterdata_radiusproximity _monsterdata_speedmultiplierattack _monsterdata_speedmultiplierescape) (break `/Game/SOUSMALINPROJET/BP/BP_Monster/S_MonsterData` (`self.MonsterData`)))
  (if (`KismetSystemLibrary.K2_IsValidTimerHandle` (`self.WaitTimer`))
    (`KismetSystemLibrary.K2_ClearAndInvalidateTimerHandle` (`self.WaitTimer`)))
  (set `self.IsAttacking` true)
  (`self.SetData`)
  (`TimelineComponent.SetPlayRate` (`self.tl_Truc`) (/ 1.0 _monsterdata_speedmultiplierattack))
  (bind (_direction _newtrack_0) (`Timeline|tl_Truc` :!label _label)
    (:`Update`
      (`self.K2_SetActorLocation` (`KismetMathLibrary.VLerp` (`self.K2_GetActorLocation`) (`self.Destination`) _newtrack_0))
      (if (`self.IsAttacking`)
        (if (> (`self.Monster Data Radius Proximity`) (`KismetMathLibrary.Vector_Distance` (`self.Destination`) (`self.K2_GetActorLocation`)))
          (`TimelineComponent.Stop` (`self.tl_Truc`))
          (bind _returnvalue (`KismetSystemLibrary.K2_SetTimerDelegate` (delegate `ECAttackSousMalin`) (`self.Monster Data Attack Cooldown`) true))
          (set `self.AttackTimer` _returnvalue))))
    (:`Finished`
      (if (not (`self.IsAttacking`))
        (`self.K2_DestroyActor`)))))

(event `ECAttackSousMalin`
  (`self.AttackSousMalin`))

(event `Escape`
  (bind (_monsterdata_radiusproximity _monsterdata_speedmultiplierattack _monsterdata_speedmultiplierescape) (break `/Game/SOUSMALINPROJET/BP/BP_Monster/S_MonsterData` (`self.MonsterData`)))
  (set `self.IsAttacking` false)
  (`TimelineComponent.SetPlayRate` (`self.tl_Truc`) (/ 1.0 _monsterdata_speedmultiplierescape))
  (goto _label :!via `Reverse`))

(event `EscapeAndWait`
  (if (`KismetSystemLibrary.K2_IsValidTimerHandle` (`self.AttackTimer`))
    (`KismetSystemLibrary.K2_ClearAndInvalidateTimerHandle` (`self.AttackTimer`)))
  (bind _returnvalue (`KismetSystemLibrary.K2_SetTimerDelegate` (delegate `ECEscape`) (`self.Monster Data Wait Cooldown`)))
  (set `self.WaitTimer` _returnvalue))

(event `ECEscape`
  (`self.Escape`))

(event `AttackSousMalin`
  (bind _asbgi_game (cast `/Game/SOUSMALINPROJET/BP/Game/BGI_Game` (`GameplayStatics.GetGameInstance`)))
  (`/Game/SOUSMALINPROJET/BP/Game/BGI_Game.OnHit` _asbgi_game))

(fn `SetData`
  (bind (_monsterdata_radiusproximity _monsterdata_speedmultiplierattack _monsterdata_speedmultiplierescape _monsterdata_attackcooldown _monsterdata_waitcooldown _monsterdata_destination) (break `/Game/SOUSMALINPROJET/BP/BP_Monster/S_MonsterData` (`self.MonsterData`)))
  (set `self.Monster Data Radius Proximity` _monsterdata_radiusproximity)
  (set `self.Monster Data Attack Cooldown` _monsterdata_attackcooldown)
  (set `self.Monster Data Wait Cooldown` _monsterdata_waitcooldown)
  (set `self.Destination` _monsterdata_destination))

(fn `UserConstructionScript`)