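; BP_Lever is a lever actor whose handle pitch is clamped between minimum and maximum amplitude every tick, starting at the minimum.
; Tick checks the handle capsule against a trigger box when inactive and a reset box when active, calling CallEDLeverPulled and playing or stopping audio on overlap.
; As wired, both branches rewrite IsLeverActive with its current value, so it stays false after BeginPlay.
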(event `self.ReceiveBeginPlay`
  (bind _handle (`self.Handle`))
  (bind (_relativerotation_roll _relativerotation_pitch _relativerotation_yaw) (`KismetMathLibrary.BreakRotator` (`SceneComponent.RelativeRotation` _handle)))
  ;[1 1 1] Initializing
  (`SceneComponent.K2_SetRelativeRotation` _handle (`KismetMathLibrary.MakeRotator` _relativerotation_roll (`self.MinAmplitude`) _relativerotation_yaw) false false)
  (set `self.IsLeverActive` false)
  (`SceneComponent.K2_SetWorldLocation` (`self.Audio`) (`self.SoundLocation`) false true))

(event `self.ReceiveTick`
  (params (DeltaSeconds :type "Float (single-precision)"))
  (bind _isleveractive (`self.IsLeverActive`))
  (bind _audio (`self.Audio`))
  (bind _handle (`self.Handle`))
  (bind (_relativerotation_roll _relativerotation_pitch _relativerotation_yaw) (`KismetMathLibrary.BreakRotator` (`SceneComponent.RelativeRotation` _handle)))
  (`|ExecutionSequence`
    (:`then_0`
      ;[1 1 1] Clamp position
      (`SceneComponent.K2_SetRelativeRotation` _handle (`KismetMathLibrary.MakeRotator` _relativerotation_roll (`KismetMathLibrary.FClamp` _relativerotation_pitch (`self.MinAmplitude`) (`self.MaxAmplitude`)) _relativerotation_yaw) false false))
    (:`then_1`
      ;[1 1 1] Update State
      (if (`self.IsLeverActive`)
        (if (`PrimitiveComponent.IsOverlappingComponent` (`self.BoxReset`) (`self.Capsule`))
          (set `self.IsLeverActive` true)
          (`self.EDLeverPulled` _isleveractive :!label _label)
          ;[1 1 1] Sound Trigger
          (if _isleveractive
            (`AudioComponent.Play` _audio 0.0)
            (else
              (`AudioComponent.Stop` _audio))))
        (elif (`PrimitiveComponent.IsOverlappingComponent` (`self.BoxTrigger`) (`self.Capsule`))
          (set `self.IsLeverActive` false)
          (goto _label))))))

(fn `UserConstructionScript`)