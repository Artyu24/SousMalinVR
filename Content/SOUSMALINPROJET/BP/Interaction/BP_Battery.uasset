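; BP_Battery is a battery grabbed with motion controllers, with a charge level shown on its mesh.
; Grabbing enables mesh physics and releases it from its current slot; functions toggle whether it can be held.
; A physics constraint links the mesh to a Cube, which snaps back to CubePosition and simulates physics on drop.
; Power-change events drive the Charge material parameter.
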(event `self.ReceiveBeginPlay`
  (bind _grabcomponent (`self.GrabComponent`))
  (add `/Game/VRTemplate/Blueprints/GrabComponent.OnGrabbed` _grabcomponent (delegate `OnGrabbed_Event`))
  (add `/Game/VRTemplate/Blueprints/GrabComponent.OnDropped` _grabcomponent (delegate `CustomEvent`))
  (`PhysicsConstraintComponent.SetConstrainedComponents` (`self.PhysicsConstraint`) (`self.Mesh`) "None" (`self.Cube`) "None")
  (add `self.OnPowerChanged` (delegate `OnPowerChanged_Event`)))

(event `OnGrabbed_Event`
  (params (`Motion controller` :type "MotionControllerComponent Object Reference"))
  (`PrimitiveComponent.SetSimulatePhysics` (`self.Mesh`) true)
  (bind _currentslot (`self.CurrentSlot`)
    (:`then`
      (`SubmarineBatterySlot.UnSlotBattery` _currentslot)
      (set `self.CurrentSlot` null))
    (:`else`)))

(event `OnPowerChanged_Event` :!signature `self.OnPowerChanged`
  (params (Value :type "Float (single-precision)"))
  (`MeshComponent.SetScalarParameterValueOnMaterials` (`self.Mesh`) "Charge" Value))

(event `CustomEvent`
  (`SceneComponent.K2_SetWorldLocation` (`self.Cube`) (`SceneComponent.K2_GetComponentLocation` (`self.CubePosition`)) false false)
  (`PrimitiveComponent.SetSimulatePhysics` (`self.Cube`) true))

(fn `DisableGrab`
  (set `/Game/VRTemplate/Blueprints/GrabComponent.BCanBeHeld` false (`self.GrabComponent`))
  (return))

(fn `EnableGrab`
  (set `/Game/VRTemplate/Blueprints/GrabComponent.BCanBeHeld` true (`self.GrabComponent`))
  (return))

(fn `UserConstructionScript`)