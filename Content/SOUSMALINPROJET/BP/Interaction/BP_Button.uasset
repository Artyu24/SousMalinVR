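; BP_Button is a pressable button that shuts down the electricity when the player pawn overlaps it.
; A press only starts while power is on, with an ActionDone flag blocking retriggers during the animation.
; A timeline slides Pivot2 along relative Y, then calls ShutDown on the ElectricitySubsystem.
; A reverse timeline animation then moves the pivot back and clears the flag on finish.
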(event `self.ReceiveBeginPlay`
  (set `self.MainPawn` (`GameplayStatics.GetPlayerPawn` 0)))

(event `self.ReceiveActorBeginOverlap`
  (params (OtherActor :type "Actor Object Reference"))
  (bind _pivot_2 (`self.Pivot_2`))
  (bind _pivot_2_2 (`self.Pivot_2`))
  (bind (_relativelocation_x _relativelocation_y _relativelocation_z) (`KismetMathLibrary.BreakVector` (`SceneComponent.RelativeLocation` _pivot_2)))
  (bind (_relativelocation_x_2 _relativelocation_y_2 _relativelocation_z_2) (`KismetMathLibrary.BreakVector` (`SceneComponent.RelativeLocation` _pivot_2_2)))
  (if (and (== OtherActor (`self.MainPawn`)) (not (`ElectricitySubsystem.bIsShutdown` (subsystem `ElectricitySubsystem`))) (not (`self.ActionDone`)))
    (set `self.ActionDone` true)
    (`KismetSystemLibrary.PrintString` "Press")
    (bind (_direction _buttonanim) (`Timeline|ButtonAnim`)
      (:`Update`
        (`SceneComponent.K2_SetRelativeLocation` _pivot_2_2 (`KismetMathLibrary.MakeVector` _relativelocation_x_2 _buttonanim _relativelocation_z_2) false false))
      (:`Finished`
        (`ElectricitySubsystem.ShutDown` (subsystem `ElectricitySubsystem`))
        (bind (_direction_2 _buttonanim_2) (`Timeline|Timeline` :!via `Reverse`)
          (:`Update`
            (`SceneComponent.K2_SetRelativeLocation` _pivot_2 (`KismetMathLibrary.MakeVector` _relativelocation_x _buttonanim_2 _relativelocation_z) false false))
          (:`Finished`
            (set `self.ActionDone` false)))))))

(fn `UserConstructionScript`)