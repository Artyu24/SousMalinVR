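; BP_SteeringWheel is a grabbable crank wheel that a motion controller turns.
; Grabbing starts a looping timer that dots the wheel's X axis with the direction to the controller, interpolating the scaled result into a local pitch step.
; Each update broadcasts the absolute value of a further interpolation through RotationValue, so listeners receive no turn direction.
; Dropping clears the controller and pauses the timer.
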(event `self.GrabComponent.OnGrabbed`
  (params (`Motion controller` :type "MotionControllerComponent Object Reference"))
  (set `self.Motion Controller` `Motion controller`)
  (bind _returnvalue (`KismetSystemLibrary.K2_SetTimerDelegate` (delegate `UpdateRotation`) 0.02 true)))

(event `UpdateRotation`
  (bind _returnvalue (`KismetMathLibrary.FInterpTo` (`self.CurrentValue`) (* (`KismetMathLibrary.Dot_VectorVector` (`KismetMathLibrary.Conv_RotatorToVector` (`KismetMathLibrary.FindLookAtRotation` (`SceneComponent.K2_GetComponentLocation` (`self.CrankWheel`)) (`SceneComponent.K2_GetComponentLocation` (`self.Motion Controller`)))) (`KismetMathLibrary.Conv_RotatorToVector` (`SceneComponent.K2_GetComponentRotation` (`self.CrankWheel`)))) 10.0) (`KismetSystemLibrary.K2_GetTimerElapsedTimeHandle` (stale `self.GrabComponent.OnGrabbed` _returnvalue)) 4.0))
  (bind _output_get (set `self.CurrentValue` _returnvalue))
  (`SceneComponent.K2_AddLocalRotation` (`self.CrankWheel`) (`KismetMathLibrary.MakeRotator` 0.0 _output_get) false false)
  (`self.RotationValue` (`KismetMathLibrary.Abs` _returnvalue)))

(event `self.GrabComponent.OnDropped`
  (set `self.Motion Controller` null)
  (`KismetSystemLibrary.K2_PauseTimer` null "UpdateRotation"))

(fn `UserConstructionScript`)