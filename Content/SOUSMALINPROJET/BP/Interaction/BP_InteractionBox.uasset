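; BP_InteractionBox is an actor with a right and a left box that follow the VR player's hands.
; On BeginPlay it caches player pawn 0 as a VRPawn.
; Every tick it copies each motion controller grip's world location and rotation to the matching box, without sweep.
; Those world values are set as relative transforms, so the boxes align only if their parent sits at the world origin, unrotated.
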(event `self.ReceiveBeginPlay`
  (bind _asvrpawn (cast `/Game/VRTemplate/Blueprints/VRPawn` (`GameplayStatics.GetPlayerPawn` 0)))
  (set `self.As VRPawn` _asvrpawn))

(event `self.ReceiveTick`
  (params (DeltaSeconds :type "Float (single-precision)"))
  (bind _motioncontrollerrightgrip (`/Game/VRTemplate/Blueprints/VRPawn.MotionControllerRightGrip` (`self.As VRPawn`)))
  (bind _motioncontrollerleftgrip (`/Game/VRTemplate/Blueprints/VRPawn.MotionControllerLeftGrip` (`self.As VRPawn`)))
  (`SceneComponent.K2_SetRelativeLocation` (`self.RightBox`) (`SceneComponent.K2_GetComponentLocation` _motioncontrollerrightgrip) false false)
  (`SceneComponent.K2_SetRelativeRotation` (`self.RightBox`) (`SceneComponent.K2_GetComponentRotation` _motioncontrollerrightgrip) false false)
  (`SceneComponent.K2_SetRelativeLocation` (`self.LeftBox`) (`SceneComponent.K2_GetComponentLocation` _motioncontrollerleftgrip) false false)
  (`SceneComponent.K2_SetRelativeRotation` (`self.LeftBox`) (`SceneComponent.K2_GetComponentRotation` _motioncontrollerleftgrip) false false))

(fn `UserConstructionScript`)