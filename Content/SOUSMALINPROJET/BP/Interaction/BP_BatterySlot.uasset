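; BP_BatterySlot is a VR interaction socket that accepts a battery when one overlaps its box while the slot is empty.
; On overlap it signals the battery change, registers itself as the battery's current slot and stores the battery.
; It then force-releases the grab, clears the VR pawn's held reference, stops the battery mesh's physics and snaps it to the slot spot.
; A connect sound plays, followed by a delayed activation sound.
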(event `self.ReceiveBeginPlay`
  (add `PrimitiveComponent.OnComponentBeginOverlap` (`self.OverlapBox`) (delegate `CustomEvent`)))

(event `CustomEvent`
  (params (OverlappedComponent :type "PrimitiveComponent Object Reference") (OtherActor :type "Actor Object Reference") (OtherComp :type "PrimitiveComponent Object Reference") (OtherBodyIndex :type Integer) (bFromSweep :type Boolean) (SweepResult :type "HitResult Structure (by ref)"))
  (bind _batteryslotspot (`self.BatterySlotSpot`))
  (`/Engine/EditorBlueprintResources/StandardMacros.IsValid` (`self.PluggedBattery`)
    (:`Is Not Valid`
      (bind _asbp_battery (cast `/Game/SOUSMALINPROJET/BP/Interaction/BP_Battery` OtherActor))
      (`self.OnBatteryChanged` _asbp_battery)
      (set `SubmarineBattery.CurrentSlot` self _asbp_battery)
      (`self.SlotBattery` _asbp_battery)
      (bind _grabcomponent (`/Game/SOUSMALINPROJET/BP/Interaction/BP_Battery.GrabComponent` _asbp_battery))
      (set `/Game/VRTemplate/Blueprints/GrabComponent.BCanBeHeld` false _grabcomponent)
      (`/Game/VRTemplate/Blueprints/GrabComponent.TryRelease` _grabcomponent)
      (`PrimitiveComponent.SetSimulatePhysics` (`SubmarineBattery.Mesh` _asbp_battery) false)
      (`PrimitiveComponent.SetSimulatePhysics` (`/Game/SOUSMALINPROJET/BP/Interaction/BP_Battery.Cube` _asbp_battery) true)
      (`self.Clear Object Held` _grabcomponent)
      (`SceneComponent.K2_SetWorldLocationAndRotation` (`SubmarineBattery.Mesh` _asbp_battery) (`SceneComponent.K2_GetComponentLocation` _batteryslotspot) (`SceneComponent.K2_GetComponentRotation` _batteryslotspot) false false)
      (`GameplayStatics.PlaySound2D` "/Game/SOUSMALINPROJET/Sound/SFX_BatteryConnectV2.SFX_BatteryConnectV2" 1.0 1.0 0.0 null null)
      (`KismetSystemLibrary.Delay` 1.0)
      (`GameplayStatics.PlaySound2D` "/Game/SOUSMALINPROJET/Sound/SFX_BatteryActivationV2.SFX_BatteryActivationV2" 1.0 1.0 0.0 null null))))

(fn `Clear Object Held`
  (params (`Grab Component` :type "/Game/VRTemplate/Blueprints/GrabComponent Object Reference"))
  (bind _asvrpawn (cast `/Game/VRTemplate/Blueprints/VRPawn` (`GameplayStatics.GetPlayerPawn` 0)))
  (if (`|EnumEquality` (`/Game/VRTemplate/Blueprints/GrabComponent.GetHeldByHand` `Grab Component`) "Left")
    (set `/Game/VRTemplate/Blueprints/VRPawn.HeldComponentLeft` null _asvrpawn)
    (else
      (set `/Game/VRTemplate/Blueprints/VRPawn.HeldComponentRight` null _asvrpawn)))
  (return))

(fn `UserConstructionScript`)